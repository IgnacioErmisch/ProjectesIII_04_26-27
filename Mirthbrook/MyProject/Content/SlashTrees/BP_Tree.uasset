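; BP_Tree is a choppable tree actor that opens a slash minigame when the player character enters its ZonaInteraccion overlap zone.
; On entry it creates and shows WBP_SlashTreeMinigame and binds its completion event, and leaving the zone removes the widget.
; Completing the minigame spawns a random number of BP_Item wood pickups scattered around the tree, then destroys it.
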(event OnComponentBeginOverlap(ZonaInteraccion)
  (params (OverlappedComponent :type Primitive%20Component%20Object%20Reference) (OtherActor :type Actor%20Object%20Reference) (OtherComp :type Primitive%20Component%20Object%20Reference) (OtherBodyIndex :type Integer) (bFromSweep :type Boolean) (SweepResult :type Hit%20Result%20Structure%20%28by%20ref%29))
  (Utilities|Casting|CastToBP_ThirdPersonCharacter OtherActor)
  (Variables|Default|SetbJugadorCerca true)
  (if (not (Variables|Default|GetbMinijuegoAbierto))
    (Variables|Default|SetbMinijuegoAbierto true)
    (bind _returnvalue (UserInterface|CreateWidget "/Game/SlashTrees/WBP_SlashTreeMinigame.WBP_SlashTreeMinigame_C" (Game|GetPlayerController 0)))
    (bind _output_get (Variables|Default|SetPanelActual _returnvalue))
    (UserInterface|Viewport|AddtoViewport _output_get 0)
    (Class|UserWidget|SetDesiredSizeinViewport _output_get "(X=300.000000,Y=500.000000)")
    (Class|UserWidget|SetPositioninViewport _output_get "(X=100.000000,Y=100.000000)" true)
    (EventDispatchers|AssignOnMinijuegoCompletado _output_get (delegate Custom|AlCompletarMinijuego))))

(event OnComponentEndOverlap(ZonaInteraccion)
  (params (OverlappedComponent :type Primitive%20Component%20Object%20Reference) (OtherActor :type Actor%20Object%20Reference) (OtherComp :type Primitive%20Component%20Object%20Reference) (OtherBodyIndex :type Integer))
  (bind _panelactual (Variables|Default|GetPanelActual))
  (Utilities|Casting|CastToBP_ThirdPersonCharacter OtherActor)
  (Variables|Default|SetbJugadorCerca false)
  (if (Variables|Default|GetbMinijuegoAbierto)
    (Utilities|IsValid _panelactual
      (:Is%20Valid
        (Widget|RemovefromParent _panelactual)
        (Variables|Default|SetbMinijuegoAbierto false)))))

(event Custom|AlCompletarMinijuego
  (bind _returnvalue (Math|Random|RandomFloatinRange -2e+02 2e+02))
  (Variables|Default|SetbMinijuegoAbierto false)
  (for _index (range 0 (- (Math|Random|RandomIntegerinRange (Variables|Default|GetMinMadera) (Variables|Default|GetMaxMadera)) 1))
    (Game|SpawnActorfromClass "/Game/Inventory/Blueprints/BP_Item.BP_Item_C" (Math|Transform|MakeTransform (+ (Transformation|GetActorLocation) (Math|Vector|MakeVector _returnvalue _returnvalue 5e+01))) "AdjustIfPossibleButAlwaysSpawn" "MultiplyWithRoot" 0 (Variables|Default|GetItemMadera) 0))
  (Actor|DestroyActor))

(event Collision|EventActorBeginOverlap
  (params (OtherActor :type Actor%20Object%20Reference)))

(event EventTick
  (params (DeltaSeconds :type Float%20%28single-precision%29)))

(fn ConstructionScript)